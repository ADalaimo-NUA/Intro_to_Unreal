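; BP_LevelPortal is an interactable trigger that moves the player to another level while persisting their progress.
; On box overlap by an actor implementing BPI_SaveLoad, it saves that actor's health plus coin data and totals from BP_CoinManager through GI_CustomGameInstance.
; It then looks up LevelToOpen in a Levels map and opens that level by name, printing an error if no entry exists.
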(event `self.ReceiveBeginPlay`
  (bind _returnvalue (`GameplayStatics.GetActorOfClass` "/Game/WorldItems/Managers/BP_CoinManager.BP_CoinManager_C"))
  (set `self.CoinManagerRef` _returnvalue))

(event `self.BoxCollider.OnComponentBeginOverlap`
  (params (OverlappedComponent :type "PrimitiveComponent Object Reference") (OtherActor :type "Actor Object Reference") (OtherComp :type "PrimitiveComponent Object Reference") (OtherBodyIndex :type Integer) (bFromSweep :type Boolean) (SweepResult :type "HitResult Structure (by ref)"))
  (bind _coinmanagerref (`self.CoinManagerRef`))
  (bind (_value _returnvalue) (`BlueprintMapLibrary.Map_Find` (`self.Levels`) (`self.LevelToOpen`)))
  ;[0 1 0 0.5] Before changing Levels, Save the Data we want to persist between Levels
  (if (`KismetSystemLibrary.DoesImplementInterface` OtherActor "/Game/GameFramework/Interfaces/BPI_SaveLoad.BPI_SaveLoad_C")
    (bind _asgi_custom_game_instance (cast `/Game/GameFramework/GI_CustomGameInstance` (`GameplayStatics.GetGameInstance`)))
    (bind _playerhealth (message `/Game/GameFramework/Interfaces/BPI_SaveLoad.FetchPlayerHealth` OtherActor))
    (`/Game/GameFramework/Interfaces/BPI_SaveLoad.SaveGame` _asgi_custom_game_instance _playerhealth (`/Game/WorldItems/Managers/BP_CoinManager.CoinData` _coinmanagerref) (`/Game/WorldItems/Managers/BP_CoinManager.TotalCoins` _coinmanagerref))
    (if _returnvalue
      (`GameplayStatics.OpenLevel` _value)
      (else
        (`KismetSystemLibrary.PrintString` "NOT A LEVEL NAME" true true (struct :`R` 1.0 :`A` 1.0) 5.0)))))

(fn `UserConstructionScript`)