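; BP_ClawMachineTrinket is a physics-simulated claw machine trinket that takes on a random look when play begins.
; SetRandomProperties rolls two independent indices to pick a material and mesh from preset arrays, storing them as MaterialValue and MeshKey to serve as the trinket's Value and Key.
; It then enables physics on the mesh, while IsInteractable always returns false.
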(event `self.ReceiveBeginPlay`
  (`self.SetRandomProperties`))

(fn `IsInteractable`
  (returns (Interactable :type Boolean))
  (return false))

(fn `SetRandomProperties`
  (bind _returnvalue (`KismetMathLibrary.RandomIntegerInRange` 0 6))
  ;[0.15 0.15 1 0.5] Sets a random Material and Mesh, using the Index values of each to set it's Key and Value properties
  (bind _output_get (set `self.MaterialValue` _returnvalue))
  (`PrimitiveComponent.SetMaterial` (`self.StaticMesh`) 0 (`|GetArrayItem` (`self.PotentialMaterials`) _output_get))
  (bind _output_get_2 (set `self.MeshKey` _returnvalue))
  (`StaticMeshComponent.SetStaticMesh` (`self.StaticMesh`) (`|GetArrayItem` (`self.PotentialMeshes`) _output_get_2))
  (`PrimitiveComponent.SetSimulatePhysics` (`self.StaticMesh`) true))

(fn `UserConstructionScript`)