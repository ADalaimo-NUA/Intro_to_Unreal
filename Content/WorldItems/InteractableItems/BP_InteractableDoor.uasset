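; Interactable door actor that swings open when an actor interacts with it, then closes itself.
; It implements Interact and always reports itself interactable, printing the interacting actor's name on use.
; The DoorOpening timeline drives DoorHinge's relative yaw, and its completion triggers CloseDoor.
; CloseDoor captures the current yaw and plays DoorClosing, adding that timeline's value as an offset.
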(event `/Game/Interfaces/BPI_Interact.Interact`
  (params (InteractingActor :type "Actor Object Reference"))
  ;[0 0.05576 1 0.5] Overridden Interface Function.
  (`KismetSystemLibrary.PrintString` (`KismetStringLibrary.Concat_StrStr` "Door Opened by: " (`KismetSystemLibrary.GetDisplayName` InteractingActor)))
  ;[0.15 1 0.03672 0.5] Door Opening set to timeline. Close Door after set Time.
  (bind (_direction _rotatevalue) (`Timeline|DoorOpening` :!via `PlayFromStart`)
    (:`Update`
      (`SceneComponent.K2_SetRelativeRotation` (`self.DoorHinge`) (`KismetMathLibrary.MakeRotator` 0.0 0.0 _rotatevalue) false false))
    (:`Finished`
      (`self.CloseDoor`))))

(event `CloseDoor`
  (bind (_relativerotation_roll _relativerotation_pitch _relativerotation_yaw) (`KismetMathLibrary.BreakRotator` (`SceneComponent.RelativeRotation` (`self.DoorHinge`))))
  ;[0.06125 0.4072 0.01521] Door Closing set to timeline. Triggered after DoorOpening has finished.
  (set `self.CurrentDoorZRotation` _relativerotation_yaw) ; Grab Current Rotation to rotate back to normal
  (bind (_direction _rotatevalue) (`Timeline|DoorClosing` :!via `PlayFromStart`)
    (:`Update`
      (`SceneComponent.K2_SetRelativeRotation` (`self.DoorHinge`) (`KismetMathLibrary.MakeRotator` 0.0 0.0 (+ (`self.CurrentDoorZRotation`) _rotatevalue)) false false))))

(fn `IsInteractable`
  (returns (Interactable :type Boolean))
  (return true))

(fn `UserConstructionScript`)