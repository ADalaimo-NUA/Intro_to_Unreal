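; BP_DamageDummy is an interactable test dummy that loses health each time an actor interacts with it.
; Interact applies a fixed base damage through UpdateHealth, which clamps health and reports death, then UpdateHealthText refreshes the text render, turning it red at low health.
; At zero health the DummyJoint rotates to show death, and further interactions only print a message.
; Despite its name, IsDummyDead returns true while health remains.
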(event `/Game/Interfaces/BPI_Interact.Interact`
  (params (InteractingActor :type "Actor Object Reference"))
  ;[0 0 1 0.5] Overridden Interact Funciton from Interface. This Actor is Damaged and health is modified.
  (`KismetSystemLibrary.PrintString` (`KismetStringLibrary.Concat_StrStr` (`KismetSystemLibrary.GetDisplayName` InteractingActor) ": Attempting to hurt Dummy"))
  ;;[0 1 0 0.5] A Check to see if Health is above 0
  (if (`self.isDummyDead`)
    (bind _isdead (`self.UpdateHealth` (`self.TakeBaseDamage`)))
    (`self.UpdateHealthText`) ; Text Renderer Component is updated \nwith updated Health
    ;;[1 0 0.3098] Dummy is 'Dead'
    ;; OPTIONAL: Add some feedback here. Maybe in a new Function/Event? DummyDeathAnim?
    (if _isdead
      (`SceneComponent.K2_SetWorldRotation` (`self.DummyJoint`) (struct :`Roll` 90.0) false false))
    (else
      (`KismetSystemLibrary.PrintString` "Dummy Dead"))))

(fn `isDummyDead`
  (returns (CanDamage :type Boolean))
  ;[0 0 1 0.5] Check if the Dummy's health is above 0 (not dead) to return if we CAN or CANNOT damage this actor
  (if (> (`self.DummyHealth`) 0)
    (return true)
    (else
      (return false))))

(fn `IsInteractable`
  (returns (Interactable :type Boolean))
  (return true))

(fn `TakeBaseDamage`
  (returns (BaseDamage :type Integer))
  ;[0 0 1 0.5] Pure Function returning a base level of damage (integer)
  (return 10))

(fn `UpdateHealth`
  (params (HealthModify :type Integer))
  (returns (isDead :type Boolean))
  ;[0 0 1 0.5] Remove the health value from our current health. If less than 0, set this actor as 'Dead' (Return True).
  ; Clamp Value to not reach bounds (0 - 100)
  (bind _output_get (set `self.DummyHealth` (`KismetMathLibrary.Clamp` (- (`self.DummyHealth`) HealthModify) 0 100)))
  (if (<= _output_get 0)
    (return true)
    (else
      (return false))))

(fn `UpdateHealthText`
  ;[0 0 1 0.5] Update Health Text. If DummyHealth is at a low value, change text Color
  (if (<= (`self.DummyHealth`) 30)
    (`TextRenderComponent.SetTextRenderColor` (`self.DummyHealthText`) (make `Color` 0 0 255)))
  (`TextRenderComponent.K2_SetText` (`self.DummyHealthText`) (`KismetTextLibrary.Conv_IntToText` (`self.DummyHealth`))))

(fn `UserConstructionScript`)