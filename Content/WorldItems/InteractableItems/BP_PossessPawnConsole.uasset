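; Interactable console that hands player control to a configured pawn, such as the claw machine pawn mentioned in its comments.
; On interact it possesses that pawn, blends the view to the console over 1.5 seconds, moves input from the interacting actor to itself and overrides the player controller's UI.
; Pressing Tab repossesses the original pawn, blends the view back and restores input and default UI.
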(event `self.Interact`
  (params (InteractingActor :type "Actor Object Reference"))
  (`/Engine/EditorBlueprintResources/StandardMacros.IsValid` (`self.PawnToPossessRef`)
    (:`Is Valid`
      (`self.PossessNewPawn` InteractingActor))
    (:`Is Not Valid`
      (`KismetSystemLibrary.PrintString` "No valid Pawn Set"))))

(event `Key|Tab`
  (params (Key :type "Key Structure"))
  (:`Pressed`
    (`self.UnpossessPawn`)))

(fn `IsInteractable`
  (returns (Interactable :type Boolean))
  (return true))

(fn `PossessNewPawn`
  (params (InteractingActorRef :type "Actor Object Reference"))
  (bind _returnvalue (`GameplayStatics.GetPlayerController` 0))
  (bind _returnvalue_2 (`GameplayStatics.GetPlayerController` 0))
  ;[0 0 1 0.5] Disable Input from interacting Actor and Posses the ClawPawn. Override current UI in PlaeyrController
  (bind _output_get (set `self.InteractingActorRef` InteractingActorRef))
  (`Controller.Possess` _returnvalue (`self.PawnToPossessRef`))
  (`PlayerController.SetViewTargetWithBlend` _returnvalue self 1.5 "VTBlend_Linear" 0.0 false)
  (`self.DisableInput` _output_get _returnvalue_2)
  (`self.EnableInput` _returnvalue_2)
  (bind _asbp_third_person_player_controller (cast `/Game/ThirdPerson/Blueprints/BP_ThirdPersonPlayerController` _returnvalue_2))
  (`/Game/ThirdPerson/Blueprints/BP_ThirdPersonPlayerController.OverrideUI` _asbp_third_person_player_controller (`self.WidgetOverride`)))

(fn `UnpossessPawn`
  (bind _returnvalue (`GameplayStatics.GetPlayerController` 0))
  (bind _returnvalue_2 (`GameplayStatics.GetPlayerController` 0))
  (bind _interactingactorref (`self.InteractingActorRef`))
  ;[0 0 1 0.5] Exit ClawMachine and Repossess the interacting Pawn. Restore Default UI back onto Player's Screen
  (`Controller.UnPossess` _returnvalue)
  (`PlayerController.SetViewTargetWithBlend` _returnvalue _interactingactorref 1.5 "VTBlend_Linear" 0.0 false)
  (bind _aspawn (cast `Pawn` _interactingactorref))
  (`Controller.Possess` _returnvalue_2 _aspawn)
  (`self.DisableInput` _returnvalue_2)
  (`self.EnableInput` (`self.InteractingActorRef`) _returnvalue_2)
  (bind _asbp_third_person_player_controller (cast `/Game/ThirdPerson/Blueprints/BP_ThirdPersonPlayerController` (`GameplayStatics.GetPlayerController` 0)))
  (`/Game/ThirdPerson/Blueprints/BP_ThirdPersonPlayerController.RestoreDefaultUI` _asbp_third_person_player_controller))

(fn `UserConstructionScript`)