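; BP_ClawPawn is a player-controlled claw machine pawn that picks up and drops interactable items.
; Movement input offsets the pawn with sweep when a line trace finds no obstruction and the claw is not lowering.
; The primary action plays a timeline that lowers the arm and triggers overlap detection, attaching one BPI_Interact actor's mesh to the grabber with physics off.
; The secondary action detaches it and restores physics.
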(event `EnhancedInput|/Game/Input/Actions/IA_Move`
  (params (ActionValue :type "Vector2D Structure") (ElapsedSeconds :type "Float (double-precision)") (TriggeredSeconds :type "Float (double-precision)") (InputAction :type "InputAction Object Reference" :default "/Game/Input/Actions/IA_Move.IA_Move"))
  (bind (_x _y) (`KismetMathLibrary.BreakVector2D` ActionValue))
  ;[0.15 0.15 1 0.5] Will line trace to the desired location before moving Claw Pawn to determine whether or not it is a viable place to move
  (:`Triggered`
    (bind _canmove (`self.AttemptMove` ActionValue))
    (if (and _canmove (not (`self.isLowering`)))
      (`self.K2_AddActorLocalOffset` (`KismetMathLibrary.MakeVector` (* _y 2.0) (* _x 2.0)) true))))

(event `EnhancedInput|/Game/Input/Actions/IA_Action`
  (params (ActionValue :type Boolean) (ElapsedSeconds :type "Float (double-precision)") (TriggeredSeconds :type "Float (double-precision)") (InputAction :type "InputAction Object Reference" :default "/Game/Input/Actions/IA_Action.IA_Action"))
  ;[0.15 0 0 0.5] Player now possesses ClawPawn. This Pawn assumes input. Action 'LMB' will lower claw arm.
  (:`Started`
    (if (and (not (`self.isLowering`)) (not (`KismetSystemLibrary.IsValid` (`self.GrabbedActor`))))
      (`self.LowerClaw`))))

(event `LowerClaw`
  ;[0 0 1 0.5] Trigger our Grabber 'ClawCollision to turn on at the bottom of the Animation
  (set `self.isLowering` true)
  (bind (_direction _z_pos_alpha) (`Timeline|ClawAnim` :!via `PlayFromStart`)
    (:`Update`
      (`SceneComponent.K2_SetRelativeLocation` (`self.ClawArm`) (`KismetMathLibrary.MakeVector` 0.0 0.0 (`KismetMathLibrary.Lerp` 0.0 -140.0 _z_pos_alpha)) false false))
    (:`Finished`
      (set `self.isLowering` false)
      (set `PrimitiveComponent.bGenerateOverlapEvents` false (`self.ClawCollision`)))
    (:`TriggerClawCollision`
      (set `PrimitiveComponent.bGenerateOverlapEvents` true (`self.ClawCollision`)))))

(event `EnhancedInput|/Game/Input/Actions/IA_SecondaryAction`
  (params (ActionValue :type Boolean) (ElapsedSeconds :type "Float (double-precision)") (TriggeredSeconds :type "Float (double-precision)") (InputAction :type "InputAction Object Reference" :default "/Game/Input/Actions/IA_SecondaryAction.IA_SecondaryAction"))
  (bind _grabbedactor (`self.GrabbedActor`))
  (bind _returnvalue (`self.GetComponentByClass` _grabbedactor "/Script/Engine.StaticMeshComponent"))
  ;[0.06125 0 0] Detach component from our Claw and reset GrabedActor Reference
  (:`Started`
    (if (and (not (`self.isLowering`)) (`KismetSystemLibrary.IsValid` _grabbedactor))
      (`SceneComponent.K2_DetachFromComponent` _returnvalue "KeepRelative" "KeepWorld" "KeepWorld" true)
      (`PrimitiveComponent.SetSimulatePhysics` _returnvalue true)
      (set `self.GrabbedActor` null))))

(event `self.ClawCollision.OnComponentBeginOverlap`
  (params (OverlappedComponent :type "PrimitiveComponent Object Reference") (OtherActor :type "Actor Object Reference") (OtherComp :type "PrimitiveComponent Object Reference") (OtherBodyIndex :type Integer) (bFromSweep :type Boolean) (SweepResult :type "HitResult Structure (by ref)"))
  ;[0.15 1 0.15 0.5] Attach Component to GrabberComponent and set SimulatePhysics to false on grabbed item so that it follows our GrabberComponent
  (if (and (`KismetSystemLibrary.DoesImplementInterface` OtherActor "/Game/GameFramework/Interfaces/BPI_Interact.BPI_Interact_C") (not (`KismetSystemLibrary.IsValid` (`self.GrabbedActor`))))
    (bind _output_get (set `self.GrabbedActor` OtherActor))
    (bind _returnvalue (`self.GetComponentByClass` _output_get "/Script/Engine.StaticMeshComponent"))
    (`PrimitiveComponent.SetSimulatePhysics` _returnvalue false)
    (`SceneComponent.K2_AttachToComponent` _returnvalue (`self.GrabberComponent`) "None" "SnapToTarget" "KeepWorld" "KeepWorld" true)))

(fn `AttemptMove`
  (params (Direction :type "Vector2D Structure"))
  (returns (CanMove :type Boolean))
  (bind _returnvalue (`self.K2_GetActorLocation`))
  ;[0.15 0.8783 0.03125 0.5] Simple Path finding on Pawn to clamp our position in an area. Look to where Player is attempting to move, is something is colliding, return false
  (bind (_outhit _returnvalue_2) (`KismetSystemLibrary.LineTraceSingle` :`Start` _returnvalue :`End` (+ (* Direction (`self.LineTraceDistance`)) _returnvalue) :`TraceChannel` "TraceTypeQuery1" :`DrawDebugType` "ForOneFrame"))
  (return (not _returnvalue_2)))

(fn `UserConstructionScript`)