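; BP_Projectile is a projectile world item that calculates and stores its own fracture strength.
; SetFractureStrength takes mass, initial velocity magnitude and time held, and stores kinetic energy (half mass times velocity squared) multiplied by time held.
; The formula is collapsed into a Math Expression node for reuse, and GetFractureStrength returns the stored value.
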(event EventSetFractureStrength
  (params (Mass :type Float%20%28double-precision%29) (InitVelocityMagnitude :type Float%20%28double-precision%29) (TimeHeld :type Float%20%28double-precision%29))
  ;[0.15 0.0774 0.02542 0.5] Task [11]: Use the values given to calculate this Actor's FractureStrength with the following formula:
  ; KineticEnergy * TimeHeld. Collapse this formula into a Math Expression in case we want to re-use later.
  (Variables|Default|SetFractureStrength (|(((0.500000*Mass)*(pow(Velocity,2)))*TimeHeld) Mass InitVelocityMagnitude TimeHeld)))

(fn ConstructionScript)

(fn GetFractureStrength
  (return (Variables|Default|GetFractureStrength)))