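; Trinket inventory container for the claw machine that collects data from trinkets entering its Box trigger.
; On overlap, it passes the trinket's mesh key and material value to AddDataToContainerType, which switches on InventoryType to fill either a Map of key-value pairs or a Set of values only.
; It then broadcasts EOnTrinketAdded with the type and both containers, intended for updating the widget in BP_ClawMachine.
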(event `self.Box.OnComponentBeginOverlap`
  (params (OverlappedComponent :type "PrimitiveComponent Object Reference") (OtherActor :type "Actor Object Reference") (OtherComp :type "PrimitiveComponent Object Reference") (OtherBodyIndex :type Integer) (bFromSweep :type Boolean) (SweepResult :type "HitResult Structure (by ref)"))
  (bind _asbp_claw_machine_trinket (cast `/Game/WorldItems/InteractableItems/BP_ClawMachineTrinket` OtherActor))
  ;[0.15 0.09675 0.01634 0.5] TASK [10]: Add new Values to Map Inventory or Set Inventory and update Widget in BP_ClawMachine via event dispatcher EOnTrinketAdded. Add the logic for this in the AddDatatoContainerType function here.
  (`self.AddDataToContainerType` (`/Game/WorldItems/InteractableItems/BP_ClawMachineTrinket.MeshKey` _asbp_claw_machine_trinket) (`/Game/WorldItems/InteractableItems/BP_ClawMachineTrinket.MaterialValue` _asbp_claw_machine_trinket))
  (`self.EOn_Trinket_Added` (`self.InventoryType`) (`self.Inventory_Map`) (`self.Inventory_Set`)))

(fn `AddDataToContainerType`
  (params (Key :type Integer) (Value :type Integer))
  ;[0.15 0.09675 0.01634 0.5] TASK [10]:Add the Key and Value properties from the Trinket Actors to the appropriate data containers depending on which 'InventoryType' this TrinketDataContainer class is.
  (switch `/Game/CustomDataTypes/Enums/Enum_TrinketInventoryType` (`self.InventoryType`)
    (:`NewEnumerator0`
      (`BlueprintMapLibrary.Map_Add` (`self.Inventory_Map`) Key Value))
    (:`NewEnumerator1`
      (`BlueprintSetLibrary.Set_Add` (`self.Inventory_Set`) Value))))

(fn `UserConstructionScript`)