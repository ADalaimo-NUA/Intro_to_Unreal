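; BP_CoinManager is a world manager that tracks the coins the player collects.
; On BeginPlay it finds every BP_Coin in the level and binds to each one's collected event.
; Each pickup increments a per-color count in a currency struct by coin type, adds its value to TotalCoins, and broadcasts an update event for the UI.
; SetCoinData lets outside code restore both values to persist them across levels.
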(event `self.ReceiveBeginPlay`
  (bind _outactors (`GameplayStatics.GetAllActorsOfClass` "/Game/WorldItems/InteractableItems/BP_Coin.BP_Coin_C"))
  (bind _output_get (set `self.Coins` _outactors)) ; Set Reference to the Coins this class will 'Manage'
  ;[0.15 0.15 1 0.5] This manager class will listen for this Event to be 'Broadcast'. It is then bound to our own event in this class to add coins to the total.
  (add `/Game/WorldItems/InteractableItems/BP_Coin.EOn_CoinCollected` _output_get (delegate `EOn_CoinCollected`)))

(event `EOn_CoinCollected`
  (params (Coin :type "/Game/WorldItems/InteractableItems/BP_Coin Object Reference") (`Coin Value` :type Integer))
  (bind (_coindata_bluecoins _coindata_greencoins _coindata_redcoins) (break `/Game/CustomDataTypes/Structs/S_CurrencyStruct` (`self.CoinData`)))
  (bind (_bluecoins _greencoins _redcoins) (break `/Game/CustomDataTypes/Structs/S_CurrencyStruct` (`self.CoinData`)))
  ;[0.15 0.15 1 0.5] This manager class will listen for this Event to be 'Broadcast'. It is then bound to our own event in this class to add coins to the total.
  ;[0 1 0 0.5] Organize the different CoinTypes into our Currency Struct. Updating as we collect Coins in the World.
  (switch `/Game/CustomDataTypes/Enums/Enum_CoinType` (`/Game/WorldItems/InteractableItems/BP_Coin.CoinType` Coin)
    (:`NewEnumerator0`
      (setmembers `/Game/CustomDataTypes/Structs/S_CurrencyStruct` :`StructRef` (`self.CoinData`) :`Blue Coins` (+ _bluecoins 1)))
    (:`NewEnumerator1`
      (setmembers `/Game/CustomDataTypes/Structs/S_CurrencyStruct` :`StructRef` (`self.CoinData`) :`Green Coins` (+ _greencoins 1)))
    (:`NewEnumerator2`
      (setmembers `/Game/CustomDataTypes/Structs/S_CurrencyStruct` :`StructRef` (`self.CoinData`) :`Red Coins` (+ _redcoins 1))))
  (`KismetSystemLibrary.PrintString` (`KismetTextLibrary.Conv_TextToString` (`|FormatText` "Blue: {b} \nGreen: {g} \nRed: {r}" _coindata_bluecoins _coindata_greencoins _coindata_redcoins)))
  (bind _output_get (set `self.TotalCoins` (+ (`self.TotalCoins`) `Coin Value`)))
  ;;[1 0 0.15 0.5] Broadcast Event for our UI to be Updated. Input TotalCoins for Correct value to be reflected.
  (`self.EOn_CoinsUpdated` _output_get))

(fn `SetCoinData`
  (params (CoinData :type "/Game/CustomDataTypes/Structs/S_CurrencyStruct Structure") (TotalCoins :type Integer))
  ;[0.15 1 0.15 0.5] Make sure Coin Data is persistent across levels
  (set `self.CoinData` CoinData)
  (set `self.TotalCoins` TotalCoins))

(fn `UserConstructionScript`)