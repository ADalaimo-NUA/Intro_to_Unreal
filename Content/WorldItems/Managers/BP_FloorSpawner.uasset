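; BP_FloorSpawner is an interactable world actor that lets the player teleport between floors.
; Interacting shows a widget and enables key 1 and 2 input until a five-second timer or leaving the box resets it.
; TransportPlayer moves the interacting actor to that floor's mapped location, activates its Data Layer, and unloads the previous one, tracking the current floor index in GI_CustomGameInstance.
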(event `self.ReceiveBeginPlay`
  (bind _asgi_custom_game_instance (cast `/Game/GameFramework/GI_CustomGameInstance` (`GameplayStatics.GetGameInstance`)))
  (set `self.GameInstanceRef` _asgi_custom_game_instance))

(event `self.Box.OnComponentEndOverlap`
  (params (OverlappedComponent :type "PrimitiveComponent Object Reference") (OtherActor :type "Actor Object Reference") (OtherComp :type "PrimitiveComponent Object Reference") (OtherBodyIndex :type Integer))
  ;[0.05299 0.15 0.03471 0.5] Either Give or Remove input from this Actor, whether or not the Player is interacting with the Spawner
  (`SceneComponent.SetVisibility` (`self.Widget`) false false)
  (`self.DisableInput` (`GameplayStatics.GetPlayerController` 0))
  (set `self.ActorRef` null))

(event `/Game/GameFramework/Interfaces/BPI_Interact.Interact`
  (params (InteractingActor :type "Actor Object Reference"))
  ;[0.05299 0.15 0.03471 0.5] Either Give or Remove input from this Actor, whether or not the Player is interacting with the Spawner
  (set `self.ActorRef` InteractingActor)
  (`SceneComponent.SetVisibility` (`self.Widget`) true false)
  (`KismetSystemLibrary.K2_SetTimerDelegate` (delegate `ResetSpawner`) 5.0)
  (`self.EnableInput` (`GameplayStatics.GetPlayerController` 0)))

(event `ResetSpawner`
  ;[0.05299 0.15 0.03471 0.5] Either Give or Remove input from this Actor, whether or not the Player is interacting with the Spawner
  (`SceneComponent.SetVisibility` (`self.Widget`) false false)
  (`self.DisableInput` (`GameplayStatics.GetPlayerController` 0))
  (set `self.ActorRef` null))

(event `Key|One`
  (params (Key :type "Key Structure"))
  ;[0.01941 0.0193 0.15 0.5] Allow player to Choose which floor to Teleport to
  (:`Pressed`
    (`self.TransportPlayer` 1)))

(event `Key|Two`
  (params (Key :type "Key Structure"))
  ;[0.01941 0.0193 0.15 0.5] Allow player to Choose which floor to Teleport to
  (:`Pressed`
    (`self.TransportPlayer` 2)))

(fn `IsInteractable`
  (returns (Interactable :type Boolean))
  (return true))

(fn `TransportPlayer`
  (params (FloorToSpawnTo :type Integer))
  (bind _currentdatalayerindex (`/Game/GameFramework/GI_CustomGameInstance.CurrentDataLayerIndex` (`self.GameInstanceRef`)))
  ;[0.15 0.1442 0.04899 0.5] If the actor Ref is valid from the interface event, move player to new Target Point in Level. Set new runtime state of data layer for new floor.
  (`/Engine/EditorBlueprintResources/StandardMacros.IsValid` (`self.ActorRef`)
    (:`Is Valid`
      (`self.DisableInput` (`GameplayStatics.GetPlayerController` 0))
      (`self.K2_SetActorLocation` (`self.ActorRef`) (`self.K2_GetActorLocation` (`BlueprintMapLibrary.Map_Find` (`self.FloorSpawnLocs`) FloorToSpawnTo)) false false)
      (`SceneComponent.SetVisibility` (`self.Widget`) false false)
      (bind _returnvalue (`WorldPartitionBlueprintLibrary.GetDataLayerManager`))
      (`DataLayerManager.SetDataLayerRuntimeState` _returnvalue (`BlueprintMapLibrary.Map_Find` (`self.DataLayersRef`) FloorToSpawnTo) "Activated" false)
      (if (!= _currentdatalayerindex (`local.FloorToSpawnTo`))
        (bind _returnvalue_2 (`DataLayerManager.SetDataLayerRuntimeState` _returnvalue (`BlueprintMapLibrary.Map_Find` (`self.DataLayersRef`) _currentdatalayerindex) "Unloaded" false))
        (if _returnvalue_2
          (set `/Game/GameFramework/GI_CustomGameInstance.CurrentDataLayerIndex` (`local.FloorToSpawnTo`) (`self.GameInstanceRef`))
          (else
            (`KismetSystemLibrary.PrintString` "Could not unload")))
        (else
          (`KismetSystemLibrary.PrintString` "Same Layer"))))
    (:`Is Not Valid`
      (`KismetSystemLibrary.PrintString` "not a valid Actor Ref"))))

(fn `UserConstructionScript`)