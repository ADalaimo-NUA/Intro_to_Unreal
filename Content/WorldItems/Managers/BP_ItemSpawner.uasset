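; BP_ItemSpawner is an interactable world actor that spawns a configurable type of item at a target's location.
; On Interact, it looks up the DT_ItemsToSpawn row named after the ItemToSpawn enum and spawns BP_ItemToSpawn once per Quantity.
; Each item gets its type, description and mesh, then its index drives SpawnCollision to handle overlapping spawns.
; IsInteractable always returns true.
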(event `/Game/GameFramework/Interfaces/BPI_Interact.Interact`
  (params (InteractingActor :type "Actor Object Reference"))
  ;[0.15 0.06023 0.02617 0.5] TASK: Using our implemented Interface BPI_Interact, spawn the Correct amount of items from our Spawner class. Modify the itemsToSpawn DataTable along with this class to spawn the appropriate amount Items
  (bind _returnvalue (`|GetDataTableRow` "/Game/CustomDataTypes/Data_Tables/DT_ItemsToSpawn.DT_ItemsToSpawn" (`KismetStringLibrary.Conv_StringToName` (`|GetEnumeratorNameAsString` (`self.ItemToSpawn`))))
    (:`then`
      (for _index (range 1 (+ (break `/Game/CustomDataTypes/Structs/S_ItemToSpawnData` _returnvalue) 1))
        (bind _returnvalue_2 (`|SpawnActorFromClass` "/Game/WorldItems/InteractableItems/BP_ItemToSpawn.BP_ItemToSpawn_C" (`KismetMathLibrary.MakeTransform` (`self.K2_GetActorLocation` (`self.SpawnTarget`))) "Undefined" "MultiplyWithRoot" null null))
        ;[0 0.000784 0.15 0.5] Helper Functions in the BP_ItemToSpawn class that will set default properties, as well as Spawn properties to help with Collision behaviours that occur when spawning multiple objects in the spame location
        (`/Game/WorldItems/InteractableItems/BP_ItemToSpawn.SetItemProperties` _returnvalue_2 (`self.ItemToSpawn`) (`.Description_17_5198D65E42495771893820A6ABBC83BB` (break `/Game/CustomDataTypes/Structs/S_ItemToSpawnData` _returnvalue)) (`.Mesh_20_B0F3E0EE4CF2EC6B1D08E1BA132866FF` (break `/Game/CustomDataTypes/Structs/S_ItemToSpawnData` _returnvalue)))
        (`/Game/WorldItems/InteractableItems/BP_ItemToSpawn.SpawnCollision` _returnvalue_2 _index)))))

(fn `IsInteractable`
  (returns (Interactable :type Boolean))
  (return true))

(fn `UserConstructionScript`)