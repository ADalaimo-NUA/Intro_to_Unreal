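; Interactable debug world item that shows a popup widget whose number buttons open one of three URLs, with FIX_ME task notes marking areas to fix or refine.
; Interact casts the actor to BP_ThirdPersonPlayerController, disables its input, and shows the widget and mouse cursor.
; Widget events bound on BeginPlay drive NumberInput, which exits and launches the matching URL, and ExitWidget, which hides the popup and restores input.
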(event `self.ReceiveBeginPlay`
  (bind _widgetref (`self.WidgetRef`))
  ;[0.15 0.07655 0 0.5] TASK [12]: FIX_ME
  ;
  ; Bind WIdget events to appropriate functions
  (add `/Game/Widgets/World/WBP_DebugBlueprintUI.On_NumberInput` _widgetref (`|CreateDelegate` :!event `[None]`))
  (add `/Game/Widgets/World/WBP_DebugBlueprintUI.On_ExitWidget` _widgetref (`|CreateDelegate` :!event `ExitWidget`)))

(event `/Game/GameFramework/Interfaces/BPI_Interact.Interact`
  (params (InteractingActor :type "Actor Object Reference"))
  ;[0.15 0.07655 0 0.5 20] TASK [12]: FIX_ME
  ;
  ; Show Widget and limit movement input from Interacting Actor
  (bind _asbp_third_person_player_controller (cast `/Game/ThirdPerson/Blueprints/BP_ThirdPersonPlayerController` InteractingActor)
    (:`then`
      (bind _output_get (set `self.ActorRef` _asbp_third_person_player_controller))
      (`self.DisableInput` _output_get (`GameplayStatics.GetPlayerController` 0))
      (`SceneComponent.SetVisibility` (`self.Widget`) true false)
      (set `PlayerController.bShowMouseCursor` true (`GameplayStatics.GetPlayerController` 0)))
    (:`CastFailed`
      (`KismetSystemLibrary.PrintString` "error: FAILED CAST TO ACTOR REF" true true (struct :`R` 1.0 :`A` 1.0) 10.0))))

(event `ExitWidget`
  ;[0.04966 0.15 0.06592 0.5] Hide Widget and give Actor back Input
  (`self.EnableInput` (`self.ActorRef`) (`GameplayStatics.GetPlayerController` 0))
  (`SceneComponent.SetVisibility` (`self.Widget`) false false)
  (set `PlayerController.bShowMouseCursor` false (`GameplayStatics.GetPlayerController` 0))
  (set `self.ActorRef` null))

(event `NumberInput`
  (params (NumInput :type Integer))
  ;[0.15 0.07655 0 0.5 20] Task [12]: FIX_ME
  ;
  ; The event bound to our Widget Popup Button Inputs. Can we refine it to clean it up / make it more readable?
  (bind _output_get (set `self.Num Input` NumInput))
  (switch `int` _output_get
    (:`Default`
      (`KismetSystemLibrary.PrintString` "error: Not a valid Number Input" false))
    (:`1`
      (`self.ExitWidget`)
      (`KismetSystemLibrary.LaunchURL` (`|GetArrayItem` (`self.URLs`))))
    (:`2`
      (`self.ExitWidget`)
      (`KismetSystemLibrary.LaunchURL` (`|GetArrayItem` (`self.URLs`) 1)))
    (:`3`
      (`self.ExitWidget`)
      (`KismetSystemLibrary.LaunchURL` (`|GetArrayItem` (`self.URLs`) 2)))))

(fn `IsInteractable`
  (returns (Interactable :type Boolean))
  (return true))

(fn `UserConstructionScript`)