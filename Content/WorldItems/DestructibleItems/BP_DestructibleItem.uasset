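; BP_DestructibleItem is a world item built on a Chaos Geometry Collection that breaks when struck.
; Actors implementing BPI_Destructible that overlap its Box supply a fracture strength, applied as a radial impulse at the collection's location.
; Strengths below the first damage threshold play a thud, while the first Chaos break event plays a break cue and starts a short lifespan before removal.
; Both sounds get randomized volume and pitch.
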(event `self.ReceiveBeginPlay`)

(event `self.Box.OnComponentBeginOverlap`
  (params (OverlappedComponent :type "PrimitiveComponent Object Reference") (OtherActor :type "Actor Object Reference") (OtherComp :type "PrimitiveComponent Object Reference") (OtherBodyIndex :type Integer) (bFromSweep :type Boolean) (SweepResult :type "HitResult Structure (by ref)"))
  (bind _geometrycollection (`self.GeometryCollection`))
  (if (`KismetSystemLibrary.DoesImplementInterface` OtherActor "/Game/GameFramework/Interfaces/BPI_Destructible.BPI_Destructible_C")
    (bind _strength (message `/Game/GameFramework/Interfaces/BPI_Destructible.GetFractureStrength` OtherActor))
    (`PhysicsObjectBlueprintLibrary.ApplyRadialImpulse` _geometrycollection (`SceneComponent.K2_GetComponentLocation` _geometrycollection) 50.0 _strength "RIF_Constant")
    (if (< _strength (`|GetArrayItem` (`GeometryCollectionComponent.DamageThreshold` _geometrycollection)))
      (`self.PlaySoundCueWithRandomProps` (`self.BoxThudCue`)))))

(event `self.GeometryCollection.OnChaosBreakEvent`
  (params (BreakEvent :type "ChaosBreakEvent Structure (by ref)"))
  (`/Engine/EditorBlueprintResources/StandardMacros.DoOnce` false
    (:`Completed`
      (`self.PlaySoundCueWithRandomProps` (`self.BoxBreakCue`))
      (`self.SetLifeSpan` 5.0))))

(fn `GetFractureStrength`
  (returns (Strength :type "Float (double-precision)"))
  (return 0.0))

(fn `UserConstructionScript`)