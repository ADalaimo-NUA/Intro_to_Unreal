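; Possessable launcher pawn that slides sideways and fires BP_Projectile, with a HUD widget shown while it is the view target.
; Movement input is gated by a line trace and applied as a swept local offset.
; Holding the action updates the widget's charge readout and triggers its animation past MaxPower.
; Release launches at VelocityMagnitude regardless of hold time, which only feeds the projectile's fracture-strength message alongside mass and velocity.
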(event `EnhancedInput|/Game/Input/Actions/IA_Move`
  (params (ActionValue :type "Vector2D Structure") (ElapsedSeconds :type "Float (double-precision)") (TriggeredSeconds :type "Float (double-precision)") (InputAction :type "InputAction Object Reference" :default "/Game/Input/Actions/IA_Move.IA_Move"))
  ;[0.15 0.15 1 0.5] Will line trace to the desired location before moving Claw Pawn to determine whether or not it is a viable place to move
  (:`Triggered`
    (bind _canmove (`self.AttemptMove` ActionValue))
    (if _canmove
      (`self.K2_AddActorLocalOffset` (`KismetMathLibrary.MakeVector` 0.0 (* (`KismetMathLibrary.BreakVector2D` ActionValue) 2.0)) true))))

(event `EnhancedInput|/Game/Input/Actions/IA_Action`
  (params (ActionValue :type Boolean) (ElapsedSeconds :type "Float (double-precision)") (TriggeredSeconds :type "Float (double-precision)") (InputAction :type "InputAction Object Reference" :default "/Game/Input/Actions/IA_Action.IA_Action"))
  (bind _launcherwidget (`self.LauncherWidget`))
  (bind _launcherwidget_2 (`self.LauncherWidget`))
  (bind _maxpower (`self.MaxPower`))
  (bind _returnvalue (* (`SceneComponent.GetForwardVector` (`self.DefaultSceneRoot`)) (`self.VelocityMagnitude`)))
  (:`Triggered`
    (`/Game/Widgets/Screen/WBP_ProjectileLauncher.SetTimeHeldText` _launcherwidget TriggeredSeconds)
    (`/Game/Widgets/Screen/WBP_ProjectileLauncher.SetFracturePercent` _launcherwidget TriggeredSeconds _maxpower)
    (if (> TriggeredSeconds _maxpower)
      (`/Engine/EditorBlueprintResources/StandardMacros.DoOnce` false :!label _label
        (:`Completed`
          (`/Game/Widgets/Screen/WBP_ProjectileLauncher.SetAnimState` (`self.LauncherWidget`) true)))))
  (:`Completed`
    (bind _returnvalue_2 (`|SpawnActorFromClass` "/Game/WorldItems/Projectiles/BP_Projectile.BP_Projectile_C" (`KismetMathLibrary.MakeTransform` (`SceneComponent.K2_GetComponentLocation` (`self.ProjectileSpawnPoint`))) "Undefined" "MultiplyWithRoot" null null))
    (bind _sphere (`/Game/WorldItems/Projectiles/BP_Projectile.Sphere` _returnvalue_2))
    (message `/Game/GameFramework/Interfaces/BPI_Destructible.SetFractureStrength` _returnvalue_2 (`PrimitiveComponent.GetMass` _sphere) (/ (`KismetMathLibrary.VSize` _returnvalue) 100.0) TriggeredSeconds)
    (bind _strength (message `/Game/GameFramework/Interfaces/BPI_Destructible.GetFractureStrength` _returnvalue_2))
    (`/Game/Widgets/Screen/WBP_ProjectileLauncher.SetFractureStrengthText` _launcherwidget_2 _strength)
    (`/Game/Widgets/Screen/WBP_ProjectileLauncher.SetAnimState` _launcherwidget_2 false)
    (`PrimitiveComponent.AddImpulse` _sphere _returnvalue "None" true)
    (goto _label :!via `Reset`)))

(event `self.K2_OnBecomeViewTarget`
  (params (PC :type "PlayerController Object Reference"))
  (bind _returnvalue (`|CreateWidget` "/Game/Widgets/Screen/WBP_ProjectileLauncher.WBP_ProjectileLauncher_C" (`GameplayStatics.GetPlayerController` 0)))
  (bind _output_get (set `self.LauncherWidget` _returnvalue))
  (`UserWidget.AddToViewport` _output_get 0))

(event `self.ReceiveUnpossessed`
  (params (OldController :type "Controller Object Reference"))
  (bind _launcherwidget (`self.LauncherWidget`))
  (`/Engine/EditorBlueprintResources/StandardMacros.IsValid` _launcherwidget
    (:`Is Valid`
      (`Widget.RemoveFromParent` _launcherwidget))))

(fn `AttemptMove`
  (params (Direction :type "Vector2D Structure"))
  (returns (CanMove :type Boolean))
  (bind _returnvalue (`self.K2_GetActorLocation`))
  ;[0.15 0.8783 0.03125 0.5] Simple Path finding on Pawn to clamp our position in an area. Look to where Player is attempting to move, is something is colliding, return false
  (bind (_outhit _returnvalue_2) (`KismetSystemLibrary.LineTraceSingle` :`Start` _returnvalue :`End` (+ (* Direction (`self.LineTraceDistance`)) _returnvalue) :`TraceChannel` "TraceTypeQuery1" :`DrawDebugType` "ForOneFrame"))
  (return (not _returnvalue_2)))

(fn `UserConstructionScript`)